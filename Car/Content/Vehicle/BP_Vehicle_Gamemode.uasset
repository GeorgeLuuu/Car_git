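; Vehicle game mode that links the simulation to an external process over a local socket connection.
; BeginPlay opens the connection, and received UTF-8 messages go to the MyVehicle actor as control data.
; Every tick it triggers line traces on all Radar actors, then sends the JSON of a single Radar back over the socket.
; Connect and disconnect handlers are empty.
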(event Custom|onConnect
  (params (SocketConnection :type Low%20Entry%20Socket%20Connection%20Object%20Reference)))

(event Custom|Receive
  (params (SocketConnection :type Low%20Entry%20Socket%20Connection%20Object%20Reference) (Bytes :type Array%20of%20Bytes))
  (bind _returnvalue (Actor|GetActorOfClass "/Game/Vehicle/MyVehicle.MyVehicle_C"))
  (Class|Vehicle|ReceiveControlData _returnvalue (Class|LowEntryExtendedStandardLibrary|BytestoStringUtf8 Bytes)))

(event Custom|OnDisconnect
  (params (SocketConnection :type Low%20Entry%20Socket%20Connection%20Object%20Reference)))

(event EventBeginPlay
  (bind _returnvalue (Class|LowEntrySocketConnectionLibrary|ConnectionCreate "127.0.0.1" 8080 (delegate Custom|onConnect) (delegate Custom|OnDisconnect) (delegate Custom|Receive)))
  (Development|PrintText "connecting")
  (Class|LowEntrySocketConnection|Connect _returnvalue)
  (Variables|Default|SetConn _returnvalue))

(event EventTick
  (params (DeltaSeconds :type Float%20%28single-precision%29))
  (bind _outactors (Actor|GetAllActorsOfClass "/Script/Car.Radar"))
  (Class|Radar|SendLineTraces _outactors 1.0)
  (Actor|GetActorOfClass 0)
  (bind _returnvalue (Actor|GetActorOfClass "/Script/Car.Radar"))
  (Class|LowEntrySocketConnection|SendMessage (Variables|Default|GetConn) (Class|LowEntryExtendedStandardLibrary|StringtoBytesUtf8 (Class|Radar|ToJsonString _returnvalue))))

(fn ConstructionScript)